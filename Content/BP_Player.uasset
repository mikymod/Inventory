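; BP_Player is a player Blueprint that owns an inventory UI and provides test input for adding items.
; On BeginPlay it creates a WBP_Inventory widget, assigns it to InventoryCharacter's Inventory, and adds it to the viewport hidden.
; Tab toggles the widget's visibility through a Select on its current state.
; Space constructs a BP_ItemTest1 object and adds it through that Inventory reference.
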(event EventBeginPlay
  (bind _returnvalue (UserInterface|CreateWidget "/Game/WBP_Inventory.WBP_Inventory_C" (Game|GetPlayerController 0)))
  (bind _output_get (Variables|Default|SetInventoryWidget _returnvalue))
  (Variables|/Script/InventoryPlugin.InventoryCharacter|SetInventory (Variables|Default|GetInventoryCharacter) _output_get)
  (UserInterface|Viewport|AddtoViewport _output_get 0)
  (Widget|SetVisibility _output_get "Hidden"))

(event Input|KeyboardEvents|Tab
  (params (Key :type Key%20Structure :default "None"))
  ;[1 1 1] Comment
  (:Pressed
    (Widget|SetVisibility (Variables|Default|GetInventoryWidget) (Utilities|Select :Index (Widget|GetVisibility (Variables|Default|GetInventoryWidget)) :Visible "Hidden" :Collapsed "Visible" :Hidden "Visible" :HitTestInvisible "Visible" :SelfHitTestInvisible "Visible"))))

(event Input|KeyboardEvents|SpaceBar
  (params (Key :type Key%20Structure :default "None"))
  (:Pressed
    (bind _returnvalue (Game|ConstructObjectfromClass "/Game/BP_ItemTest1.BP_ItemTest1_C"))
    (Class|Inventory|AddItem (Variables|/Script/InventoryPlugin.InventoryCharacter|GetInventory (Variables|Default|GetInventoryCharacter)) _returnvalue)))

(fn ConstructionScript)